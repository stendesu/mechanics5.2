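; BP_Starter_Weapon is the starter weapon for a tank, firing projectiles from the owning tank.
; When started, it spawns a BP_Projectile at the location and rotation of MyTank's DirectionArrow, provided it is not on cooldown.
; Each shot sets a Cooldown flag that a short one-shot timer clears, limiting the fire rate.
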(event Custom|EndCooldown
  ;[1 1 1] Weapon Cooldown
  (Variables|Default|Setcooldown false))

(event Custom|OnCooldown
  ;[1 1 1] Weapon Cooldown
  (Variables|Default|Setcooldown true)
  (Utilities|Time|SetTimerbyEvent (delegate Custom|EndCooldown) 0.4))

(event EventStarted
  (bind _mytank (Variables|Default|GetMyTank))
  (bind _directionarrow (Variables|/Game/Blueprints/BP_PlayerCharacter.BP_PlayerCharacter_C|GetDirectionArrow _mytank))
  (if (not (Variables|Default|Getcooldown))
    (Game|SpawnActorfromClass "/Game/StudentWork/PlayerProjectiles/BP_Projectile.BP_Projectile_C" (Math|Transform|MakeTransform (Transformation|GetWorldLocation _directionarrow) (Transformation|GetWorldRotation _directionarrow) "1.000000,1.000000,1.000000") "Undefined" "MultiplyWithRoot" 0 0)
    (CallFunction|OnCooldown)))

(fn ConstructionScript
  (|CallParentFunction))