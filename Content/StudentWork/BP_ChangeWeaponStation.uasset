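; Weapon change station actor that lets the player use the weapon menu while standing in its interactable range.
; A Sphere overlap caches the player, and Tick then turns the Widget toward that player's camera with a look-at rotation and flipped yaw.
; Entering InteractableRange enables the player's weapon menu and UI mode, and leaving it calls SetToGameMode.
; An unconnected leftover block holds the manual menu collapse and flag reset.
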(event OnComponentBeginOverlap(Sphere)
  (params (OverlappedComponent :type Primitive%20Component%20Object%20Reference) (OtherActor :type Actor%20Object%20Reference) (OtherComp :type Primitive%20Component%20Object%20Reference) (OtherBodyIndex :type Integer) (bFromSweep :type Boolean) (SweepResult :type Hit%20Result%20Structure%20%28by%20ref%29))
  (bind _asbp_player_character (Utilities|Casting|CastToBP_PlayerCharacter OtherActor))
  (Variables|Default|SetPlayerRef _asbp_player_character))

(event OnComponentBeginOverlap(interactableRange)
  (params (OverlappedComponent :type Primitive%20Component%20Object%20Reference) (OtherActor :type Actor%20Object%20Reference) (OtherComp :type Primitive%20Component%20Object%20Reference) (OtherBodyIndex :type Integer) (bFromSweep :type Boolean) (SweepResult :type Hit%20Result%20Structure%20%28by%20ref%29))
  (bind _asbp_player_character (Utilities|Casting|CastToBP_PlayerCharacter OtherActor))
  (bind _output_get (Variables|Default|SetPlayerRef _asbp_player_character))
  (Variables|/Game/Blueprints/BP_PlayerCharacter.BP_PlayerCharacter_C|SetenableWeaponMenu _output_get true)
  (Variables|/Game/Blueprints/BP_PlayerCharacter.BP_PlayerCharacter_C|SetUIMode _output_get true))

(event OnComponentEndOverlap(interactableRange)
  (params (OverlappedComponent :type Primitive%20Component%20Object%20Reference) (OtherActor :type Actor%20Object%20Reference) (OtherComp :type Primitive%20Component%20Object%20Reference) (OtherBodyIndex :type Integer))
  (bind _asbp_player_character (Utilities|Casting|CastToBP_PlayerCharacter OtherActor))
  (bind _output_get (Variables|Default|SetPlayerRef _asbp_player_character))
  (Default|SettoGameMode _output_get))

(event EventTick
  (params (DeltaSeconds :type Float%20%28single-precision%29))
  (bind _widget (Variables|Default|GetWidget))
  ;[1 1 1] Comment
  (bind _playerref (Variables|Default|GetPlayerRef)
    (:then
      (Transformation|SetWorldRotation _widget (Math|Rotator|MakeRotator (.roll (Math|Rotator|FindLookatRotation (Transformation|GetWorldLocation (Variables|/Game/Blueprints/BP_PlayerCharacter.BP_PlayerCharacter_C|GetCamera _playerref)) (Transformation|GetWorldLocation _widget))) (.pitch (Math|Rotator|FindLookatRotation (Transformation|GetWorldLocation (Variables|/Game/Blueprints/BP_PlayerCharacter.BP_PlayerCharacter_C|GetCamera _playerref)) (Transformation|GetWorldLocation _widget))) (+ (.yaw (Math|Rotator|FindLookatRotation (Transformation|GetWorldLocation (Variables|/Game/Blueprints/BP_PlayerCharacter.BP_PlayerCharacter_C|GetCamera _playerref)) (Transformation|GetWorldLocation _widget))) 1.8e+02)) false false))
    (:else)))

(fn ConstructionScript)