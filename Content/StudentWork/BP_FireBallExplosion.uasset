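; Fireball explosion actor that spawns a Niagara explosion effect and deals area damage on overlap.
; Two overlap components form damage zones, with Inner applying 1.5x the Damage variable and Outer 0.3x.
; Every tick it plays a world camera shake centered on the player character's location rather than the explosion's, so distance from the blast does not attenuate it.
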(event OnComponentBeginOverlap(Outer)
  (params (OverlappedComponent :type Primitive%20Component%20Object%20Reference) (OtherActor :type Actor%20Object%20Reference) (OtherComp :type Primitive%20Component%20Object%20Reference) (OtherBodyIndex :type Integer) (bFromSweep :type Boolean) (SweepResult :type Hit%20Result%20Structure%20%28by%20ref%29))
  ;[1 1 1] deal damage
  (Game|Damage|ApplyDamage OtherActor (* (Variables|Default|GetDamage) 0.3) 0 0))

(event OnComponentBeginOverlap(Inner)
  (params (OverlappedComponent :type Primitive%20Component%20Object%20Reference) (OtherActor :type Actor%20Object%20Reference) (OtherComp :type Primitive%20Component%20Object%20Reference) (OtherBodyIndex :type Integer) (bFromSweep :type Boolean) (SweepResult :type Hit%20Result%20Structure%20%28by%20ref%29))
  ;[1 1 1] deal damage
  (Game|Damage|ApplyDamage OtherActor (* (Variables|Default|GetDamage) 1.5) 0 0))

(event EventBeginPlay
  ;[1 1 1] spawn eeffect
  (Niagara|SpawnSystematLocation "/Game/StudentWork/vfx/NS_Explosion.NS_Explosion" (Transformation|GetActorLocation) "0, 0, 0" "1.300000,1.300000,1.300000"))

(event EventTick
  (params (DeltaSeconds :type Float%20%28single-precision%29))
  ;[1 1 1] play camera shake
  (bind _asbp_player_character (Utilities|Casting|CastToBP_PlayerCharacter (Game|Player|GetPlayerPawn 0)))
  (Camera|PlayWorldCameraShake "/Game/StudentWork/CameraShakes/CS_Explosion.CS_Explosion_C" (Transformation|GetActorLocation _asbp_player_character) 0.0 3e+03 1e+01 true))

(fn ConstructionScript)