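; BP_Test is a test enemy Blueprint that runs a simple state machine on Tick.
; Each frame it prints the current state on screen.
; In the moving state it calls AI MoveTo and switches to the next state on reaching the stopping distance.
; The attack and idle branches are empty, and the Move event is an unused stub.
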(event Custom|Event%20Move)

(event EventTick
  (params (DeltaSeconds :type Float%20%28single-precision%29))
  (Utilities|FlowControl|Sequence
    (:then_0
      (Development|PrintString (Utilities|String|ToString(Text) (Utilities|Text|FormatText "enemy current state = {X}" (Utilities|String|EnumtoString (Variables|Default|GetcurrentState)))) true true "(R=0.000000,G=0.660000,B=1.000000,A=1.000000)" 0.001))
    (:then_1
      (if (Utilities|Enum|Equal(Enum) (Variables|Default|GetcurrentState) "NewEnumerator2")
        ;[1 1 1] Comment
        (AI|AIMoveTo 0 "0, 0, 0" 0 (Variables|Default|GetStoppingDistance) false
          (:then)
          (:OnSuccess
            ;;[1 1 1] reaches destination stopping distance
            (Variables|Default|SetcurrentState "NewEnumerator1")))
        (elif (not (Utilities|Enum|Equal(Enum) (Variables|Default|GetcurrentState) "NewEnumerator1"))
          (if (Utilities|Enum|Equal(Enum) (Variables|Default|GetcurrentState) "NewEnumerator0")
            _))))))

(fn ConstructionScript)