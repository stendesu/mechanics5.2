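; Timed lightning-storm area that expands, spawns BP_LightningBolt actors on random targets within it, then shrinks and destroys itself after about ten seconds.
; A state enum sequences the phases, with the ExpandMesh timeline scaling the main and decor components in and out.
; While active, Tick runs a box trace and a Delay paces strikes at random hit actors' locations.
; SetDurationBasedOnIndex supplies that delay, though its hit-count formula appears unconnected.
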(event Custom|BeginLightningEvent
  (bind _returnvalue (Transformation|GetActorLocation))
  (Utilities|FlowControl|Sequence
    (:then_0
      (Utilities|FlowControl|DoOnce false
        (:Completed
          (Utilities|FlowControl|Delay 1e+01)
          (Variables|Default|SetStates "NewEnumerator2")
          (bind _scale (Timeline|ExpandMesh ReverseFromEnd)
            (:Update
              (Transformation|SetRelativeScale3D (Variables|Default|GetMain) (Math|Vector|Lerp(Vector) "0, 0, 0" "6.000000,6.000000,0.500000" _scale))
              (Transformation|SetRelativeScale3D (Variables|Default|GetDecor2) (/ (Math|Vector|Lerp(Vector) "0, 0, 0" "6.000000,6.000000,0.500000" _scale) "2.100000,2.100000,1.000000"))
              (Transformation|SetRelativeScale3D (Variables|Default|GetDecor5) (/ (Math|Vector|Lerp(Vector) "0, 0, 0" "6.000000,6.000000,0.500000" _scale) "2.000000,2.000000,1.000000")))
            (:Finished
              (if (Utilities|Enum|Equal(Enum) (Variables|Default|GetStates) "NewEnumerator0")
                (Variables|Default|SetStates "NewEnumerator1")
                (elif (Utilities|Enum|Equal(Enum) (Variables|Default|GetStates) "NewEnumerator2")
                  (Actor|DestroyActor))))))))
    (:then_1
      (bind _outhits (Class|KismetSystemLibrary|BoxTraceMultiforObjects _returnvalue _returnvalue "600.000000,600.000000,1000.000000" "0, 0, 0" (Variables|Default|GetObject%20Types) false 0 "ForOneFrame" true))
      (Utilities|FlowControl|Delay (Utilities|SetDurationBasedonIndex _outhits))
      (Utilities|IsValid (.HitActor (Collision|BreakHitResult (.OutItem (Utilities|Array|Random _outhits))))
        (:Is%20Valid
          (Game|SpawnActorfromClass "/Game/StudentWork/BP_LightningBolt.BP_LightningBolt_C" (Math|Transform|MakeTransform (Transformation|GetActorLocation (.HitActor (Collision|BreakHitResult (.OutItem (Utilities|Array|Random _outhits))))) (Math|Rotator|MakeRotator 0.0 0.0 (Math|Random|RandomFloatinRange 0.0 3.6e+02)) "1.000000,1.000000,1.000000") "Undefined" "MultiplyWithRoot" 0 0))))))

(event EventBeginPlay
  (Variables|Default|SetStates "NewEnumerator0")
  (bind _scale (Timeline|ExpandMesh PlayFromStart)
    (:Update
      (Transformation|SetRelativeScale3D (Variables|Default|GetMain) (Math|Vector|Lerp(Vector) "0, 0, 0" "6.000000,6.000000,0.500000" _scale))
      (Transformation|SetRelativeScale3D (Variables|Default|GetDecor2) (/ (Math|Vector|Lerp(Vector) "0, 0, 0" "6.000000,6.000000,0.500000" _scale) "2.100000,2.100000,1.000000"))
      (Transformation|SetRelativeScale3D (Variables|Default|GetDecor5) (/ (Math|Vector|Lerp(Vector) "0, 0, 0" "6.000000,6.000000,0.500000" _scale) "2.000000,2.000000,1.000000")))
    (:Finished
      (if (Utilities|Enum|Equal(Enum) (Variables|Default|GetStates) "NewEnumerator0")
        (Variables|Default|SetStates "NewEnumerator1")
        (elif (Utilities|Enum|Equal(Enum) (Variables|Default|GetStates) "NewEnumerator2")
          (Actor|DestroyActor))))))

(event EventTick
  (params (DeltaSeconds :type Float%20%28single-precision%29))
  (if (Utilities|Enum|Equal(Enum) (Variables|Default|GetStates) "NewEnumerator1")
    (CallFunction|BeginLightningEvent)))

(fn ConstructionScript)