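; BP_HealthPackSpawner is an actor that spawns a health pack and replaces it once it leaves the spawner's box.
; BeginPlay and the box's end-overlap with a BP_HealthPack both start the slowed FadeToGreen timeline.
; The timeline drives FlashLevel on a dynamic material created in the construction script, then spawns a new pack at SpawnPoint when finished.
; The timeline therefore times respawns; the PackRespawnRate delay is unconnected.
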(event OnComponentEndOverlap(Box)
  (params (OverlappedComponent :type Primitive%20Component%20Object%20Reference) (OtherActor :type Actor%20Object%20Reference) (OtherComp :type Primitive%20Component%20Object%20Reference) (OtherBodyIndex :type Integer))
  ;[1 1 1] Repsawn healthpack when taken
  (Utilities|Casting|CastToBP_HealthPack OtherActor)
  (CallFunction|TriggerTimeline))

(event Custom|spawnHealthPack
  ;[1 1 1] Spawn pack
  (bind _returnvalue (Game|SpawnActorfromClass "/Game/StudentWork/BP_HealthPack.BP_HealthPack_C" (Transformation|GetWorldTransform (Variables|Default|GetspawnPoint)) "Undefined" "MultiplyWithRoot" 0 0))
  (Variables|Default|SetspawnedHealthPack _returnvalue))

(event Custom|TriggerTimeline
  ;[1 1 1] Mat tl
  (bind _fadeto (Timeline|FadeToGreen PlayFromStart)
    (:Update
      (Rendering|Material|SetScalarParameterValue (Variables|Default|GetFlashMat) "FlashLevel" _fadeto :!class /Script/Engine.MaterialInstanceDynamic))
    (:Finished
      (CallFunction|SpawnHealthPack))))

(event Custom|ResetMat
  ;[1 1 1] Mat tl
  (bind _fadeto (Timeline|FadeToGreen Reverse)
    (:Update
      (Rendering|Material|SetScalarParameterValue (Variables|Default|GetFlashMat) "FlashLevel" _fadeto :!class /Script/Engine.MaterialInstanceDynamic))
    (:Finished
      (CallFunction|SpawnHealthPack))))

(event EventBeginPlay
  ;[1 1 1] initialize
  (Components|Timeline|SetPlayRate (Variables|Default|GetFadeToGreen) 0.33)
  (CallFunction|TriggerTimeline))

(fn ConstructionScript
  (bind _returnvalue (Rendering|Material|CreateDynamicMaterialInstance (Variables|Default|GetStaticMesh1) 0 "/Game/StudentWork/Materials/M_FadeFlash.M_FadeFlash" "None" :!class /Script/Engine.PrimitiveComponent))
  (Variables|Default|SetFlashMat _returnvalue))