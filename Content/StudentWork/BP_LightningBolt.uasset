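; Lightning bolt actor that spawns a Niagara impact effect at its location on BeginPlay and damages what it touches.
; Every Tick it plays an explosion world camera shake centered on the player character rather than on the bolt.
; Its sphere overlap applies fixed damage to any overlapping actor and first sets a status enum on those that are BP_EnemyParent.
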(event OnComponentBeginOverlap(Sphere)
  (params (OverlappedComponent :type Primitive%20Component%20Object%20Reference) (OtherActor :type Actor%20Object%20Reference) (OtherComp :type Primitive%20Component%20Object%20Reference) (OtherBodyIndex :type Integer) (bFromSweep :type Boolean) (SweepResult :type Hit%20Result%20Structure%20%28by%20ref%29))
  ;[1 1 1] deal damage
  (bind _output_get (Variables|Default|SetDamaged%20Actor OtherActor))
  (bind _asbp_enemy_parent (Utilities|Casting|CastToBP_EnemyParent _output_get)
    (:then
      (Variables|/Game/StudentWork/Enemy/BP_EnemyParent.BP_EnemyParent_C|SetCurrent%20Status _asbp_enemy_parent "NewEnumerator3"))
    (:CastFailed
      _))
  (Game|Damage|ApplyDamage _output_get 35.0 0 0))

(event EventBeginPlay
  ;[1 1 1] spawn eeffect
  (Niagara|SpawnSystematLocation "/Game/StudentWork/vfx/NS_LightningImpact.NS_LightningImpact" (Transformation|GetActorLocation)))

(event EventTick
  (params (DeltaSeconds :type Float%20%28single-precision%29))
  ;[1 1 1] play camera shake
  (bind _asbp_player_character (Utilities|Casting|CastToBP_PlayerCharacter (Game|Player|GetPlayerPawn 0)))
  (Camera|PlayWorldCameraShake "/Game/StudentWork/CameraShakes/CS_Explosion.CS_Explosion_C" (Transformation|GetActorLocation _asbp_player_character) 0.0 3e+03 25.0 true))

(fn ConstructionScript)