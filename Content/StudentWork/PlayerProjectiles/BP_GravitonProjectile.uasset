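; Graviton player projectile that each frame looks for nearby enemies and sets their location, apparently meant as a gravity pull.
; Tick runs a debug-drawn sphere trace around the projectile and teleport-free, unswept moves each BP_EnemyParent hit to FindDistanceAndAddLocation's result.
; That function holds PullForce-scaled, delta-time math toward the projectile, but it is left unused.
; BeginPlay destroys ProjectileMovement after a short delay, halting the projectile.
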(event EventTick
  (params (DeltaSeconds :type Float%20%28single-precision%29))
  (bind _returnvalue (Transformation|GetActorLocation))
  (bind _outhits (Collision|MultiSphereTraceForObjects _returnvalue _returnvalue 1.3e+03 (Variables|Default|GetObject%20Types) false 0 "ForOneFrame"))
  (for _array_element _outhits
    (bind _asbp_enemy_parent (Utilities|Casting|CastToBP_EnemyParent (.HitActor (Collision|BreakHitResult _array_element))))
    (Transformation|SetActorLocation _asbp_enemy_parent (Utilities|FindDistanceandAddLocation _asbp_enemy_parent) false false)))

(event EventBeginPlay
  (Utilities|FlowControl|Delay 2.0)
  (Components|DestroyComponent (Variables|Default|GetProjectileMovement)))

(fn ConstructionScript)