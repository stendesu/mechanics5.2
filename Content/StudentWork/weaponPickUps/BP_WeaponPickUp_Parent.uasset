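; BP_WeaponPickUp_Parent is a parent weapon pickup that gives the player a new weapon on overlap.
; On BeginPlay it tints its point light with a configurable color.
; When a BP_PlayerCharacter enters its box, it spawns the configured Weapon class far below the origin.
; It passes that BP_BaseWeapon_Parent to the character's LinkNewWeapon, then destroys itself.
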(event OnComponentBeginOverlap(Box)
  (params (OverlappedComponent :type Primitive%20Component%20Object%20Reference) (OtherActor :type Actor%20Object%20Reference) (OtherComp :type Primitive%20Component%20Object%20Reference) (OtherBodyIndex :type Integer) (bFromSweep :type Boolean) (SweepResult :type Hit%20Result%20Structure%20%28by%20ref%29))
  ;[1 1 1] When the Player Collides, update their existing weapon with the new one, then destroy this pick up
  (bind _asbp_player_character (Utilities|Casting|CastToBP_PlayerCharacter OtherActor))
  (bind _returnvalue (Game|SpawnActorfromClass (Variables|Default|GetWeapon) (Math|Transform|MakeTransform "0.000000,0.000000,-5000.000000" "0, 0, 0" "1.000000,1.000000,1.000000") "Undefined" "MultiplyWithRoot" 0 0))
  (bind _asbp_base_weapon_parent (Utilities|Casting|CastToBP_BaseWeapon_Parent _returnvalue))
  (Default|LinkNewWeapon _asbp_player_character _asbp_base_weapon_parent)
  (Actor|DestroyActor))

(event EventBeginPlay
  (Rendering|Components|Light|SetLightColor (Variables|Default|GetPointLight) (Variables|Default|GetNew%20Light%20Color) true))

(fn ConstructionScript
  (|CallParentFunction))