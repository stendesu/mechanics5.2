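; BP_target is a destructible target actor that flashes and then explodes after taking any damage.
; The construction script creates a dynamic instance of M_FlashingTL on its static mesh.
; The first damage event, gated by a DoOnce, plays a timeline driving that material's FlashLevel parameter.
; When the timeline finishes, it spawns BP_NaturalExplosion, then destroys itself and spawns the NS_Explosion Niagara effect at its location.
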(event Custom|SpawnExplosion
  (Game|SpawnActorfromClass "/Game/StudentWork/BP_NaturalExplosion.BP_NaturalExplosion_C" (Transformation|GetActorTransform) "Undefined" "MultiplyWithRoot" 0 0))

(event Custom|deathevent
  ;[1 1 1] Comment
  (Actor|DestroyActor)
  (Niagara|SpawnSystematLocation "/Game/StudentWork/vfx/NS_Explosion.NS_Explosion" (Transformation|GetActorLocation)))

(event Game|Damage|EventAnyDamage
  (params (Damage :type Float%20%28single-precision%29) (DamageType :type Damage%20Type%20Object%20Reference) (InstigatedBy :type Controller%20Object%20Reference) (DamageCauser :type Actor%20Object%20Reference))
  (Utilities|FlowControl|DoOnce false
    (:Completed
      (bind _flash (Timeline|Flash PlayFromStart)
        (:Update
          (Rendering|Material|SetScalarParameterValue (Variables|Default|GetFlashMaterial) "FlashLevel" _flash :!class /Script/Engine.MaterialInstanceDynamic))
        (:Finished
          (CallFunction|SpawnExplosion)
          (CallFunction|Deathevent))))))

(fn ConstructionScript
  (bind _returnvalue (Rendering|Material|CreateDynamicMaterialInstance (Variables|Default|GetStaticMesh) 0 "/Game/StudentWork/Materials/M_FlashingTL.M_FlashingTL" "None" :!class /Script/Engine.PrimitiveComponent))
  (Variables|Default|SetFlashMaterial _returnvalue))