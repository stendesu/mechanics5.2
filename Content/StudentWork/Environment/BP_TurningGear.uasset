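; BP_TurningGear is an environment actor that spins a gear mesh continuously.
; On BeginPlay it assigns the GearMesh variable to its StaticMesh component.
; Each Tick adds relative yaw using TurnRate, or TurnRateReverse when the Reverse flag is set.
; The rotation is not scaled by delta time, so spin speed depends on frame rate.
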(event EventBeginPlay
  (Components|StaticMesh|SetStaticMesh (Variables|Default|GetStaticMesh) (Variables|Default|GetgearMesh)))

(event EventTick
  (params (DeltaSeconds :type Float%20%28single-precision%29))
  (bind _staticmesh (Variables|Default|GetStaticMesh))
  (if (Variables|Default|Getreverse?)
    (Transformation|AddRelativeRotation _staticmesh (Math|Rotator|MakeRotator 0.0 0.0 (Variables|Default|GetturnRateReverse)) false false)
    (else
      (Transformation|AddRelativeRotation _staticmesh (Math|Rotator|MakeRotator 0.0 0.0 (Variables|Default|GetturnRate)) false false))))

(fn ConstructionScript)