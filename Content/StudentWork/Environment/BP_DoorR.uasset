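; BP_DoorR is a sliding door that opens automatically when the player character approaches.
; On BeginPlay it stores its start position and an open position offset along its right vector.
; Box overlap begin and end with BP_PlayerCharacter call OpenDoor and CloseDoor, which play and reverse a Timeline.
; The Timeline track lerps the actor's location between the two positions, so the whole actor moves.
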(event OnComponentBeginOverlap(Box)
  (params (OverlappedComponent :type Primitive%20Component%20Object%20Reference) (OtherActor :type Actor%20Object%20Reference) (OtherComp :type Primitive%20Component%20Object%20Reference) (OtherBodyIndex :type Integer) (bFromSweep :type Boolean) (SweepResult :type Hit%20Result%20Structure%20%28by%20ref%29))
  (Utilities|Casting|CastToBP_PlayerCharacter OtherActor)
  (CallFunction|OpenDoor))

(event OnComponentEndOverlap(Box)
  (params (OverlappedComponent :type Primitive%20Component%20Object%20Reference) (OtherActor :type Actor%20Object%20Reference) (OtherComp :type Primitive%20Component%20Object%20Reference) (OtherBodyIndex :type Integer))
  (Utilities|Casting|CastToBP_PlayerCharacter OtherActor)
  (CallFunction|CloseDoor))

(event Custom|CloseDoor
  (bind _track1 (Timeline|Timeline Reverse)
    (:Update
      (Transformation|SetActorLocation (Math|Vector|Lerp(Vector) (Variables|Default|GetstartLocation) (Variables|Default|GetopenLocation) _track1) false false))))

(event Custom|OpenDoor
  (bind _track1 (Timeline|Timeline Play)
    (:Update
      (Transformation|SetActorLocation (Math|Vector|Lerp(Vector) (Variables|Default|GetstartLocation) (Variables|Default|GetopenLocation) _track1) false false))))

(event EventBeginPlay
  (Variables|Default|SetstartLocation (Transformation|GetActorLocation))
  (Variables|Default|SetopenLocation (+ (Transformation|GetActorLocation) (* (Transformation|GetActorRightVector) 2e+02))))

(fn ConstructionScript)