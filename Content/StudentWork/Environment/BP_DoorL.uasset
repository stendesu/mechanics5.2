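; BP_DoorL is a sliding door that opens while the player character is inside its trigger box and closes when they leave.
; On BeginPlay it stores its start location and an open location offset along the negative right vector.
; Box overlap events, filtered by a cast to BP_PlayerCharacter, play or reverse a Timeline whose track lerps the actor between those two locations.
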(event OnComponentBeginOverlap(Box)
  (params (OverlappedComponent :type Primitive%20Component%20Object%20Reference) (OtherActor :type Actor%20Object%20Reference) (OtherComp :type Primitive%20Component%20Object%20Reference) (OtherBodyIndex :type Integer) (bFromSweep :type Boolean) (SweepResult :type Hit%20Result%20Structure%20%28by%20ref%29))
  ;[1 1 1] ManageOverlap
  (Utilities|Casting|CastToBP_PlayerCharacter OtherActor)
  (CallFunction|OpenDoor))

(event OnComponentEndOverlap(Box)
  (params (OverlappedComponent :type Primitive%20Component%20Object%20Reference) (OtherActor :type Actor%20Object%20Reference) (OtherComp :type Primitive%20Component%20Object%20Reference) (OtherBodyIndex :type Integer))
  ;[1 1 1] ManageOverlap
  (Utilities|Casting|CastToBP_PlayerCharacter OtherActor)
  (CallFunction|CloseDoor))

(event Custom|CloseDoor
  ;[1 1 1] Timeline
  (bind _track1 (Timeline|Timeline Reverse)
    (:Update
      (Transformation|SetActorLocation (Math|Vector|Lerp(Vector) (Variables|Default|GetstartLocation) (Variables|Default|GetopenLocation) _track1) false false))))

(event Custom|OpenDoor
  ;[1 1 1] Timeline
  (bind _track1 (Timeline|Timeline Play)
    (:Update
      (Transformation|SetActorLocation (Math|Vector|Lerp(Vector) (Variables|Default|GetstartLocation) (Variables|Default|GetopenLocation) _track1) false false))))

(event EventBeginPlay
  ;[1 1 1] SetValue
  (Variables|Default|SetstartLocation (Transformation|GetActorLocation))
  (Variables|Default|SetopenLocation (+ (Transformation|GetActorLocation) (* (Transformation|GetActorRightVector) -5e+02))))

(fn ConstructionScript)