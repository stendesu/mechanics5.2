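; Rifle weapon for the player's tank that fires a BP_RifleProjectile whenever it is triggered outside of cooldown.
; Each shot spawns at the tank's DirectionArrow, adding MakeSpread's pitch and yaw to the arrow's rotation.
; The makeSpread graph builds a small random rotator scaled by the tank's EnableRecoil.
; Firing sets a Cooldown flag that a one-shot timer clears after FireRate seconds.
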(event Custom|EndCooldown
  ;[1 1 1] Weapon Cooldown
  (Variables|Default|Setcooldown false))

(event Custom|OnCooldown
  ;[1 1 1] Weapon Cooldown
  (Variables|Default|Setcooldown true)
  (Utilities|Time|SetTimerbyEvent (delegate Custom|EndCooldown) (Variables|Default|GetfireRate)))

(event Custom|FiringEvent
  (bind _returnvalue (Utilities|MakeSpread))
  (bind _mytank (Variables|Default|GetMyTank))
  (bind _directionarrow (Variables|/Game/Blueprints/BP_PlayerCharacter.BP_PlayerCharacter_C|GetDirectionArrow _mytank))
  (bind _returnvalue_2 (Transformation|GetWorldRotation _directionarrow))
  ;[1 1 1] Firing Event
  (CallFunction|OnCooldown)
  (Game|SpawnActorfromClass "/Game/StudentWork/PlayerProjectiles/BP_RifleProjectile.BP_RifleProjectile_C" (Math|Transform|MakeTransform (Transformation|GetWorldLocation _directionarrow) (Math|Rotator|MakeRotator 0.0 (+ (.pitch _returnvalue_2) (.pitch _returnvalue)) (+ (.yaw _returnvalue_2) (.yaw _returnvalue))) "1.000000,1.000000,1.000000") "Undefined" "MultiplyWithRoot" 0 0))

(event EventBeginPlay)

(event EventTriggered
  (if (not (Variables|Default|Getcooldown))
    (CallFunction|FiringEvent)))

(fn ConstructionScript
  (|CallParentFunction))