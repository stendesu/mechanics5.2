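; BP_FlameWeapon is a tank flamethrower that damages what it hits in a short range ahead of the tank's DirectionArrow.
; Input start attaches a Niagara fire effect to the arrow, and completion deactivates it.
; While triggered, a timer-based cooldown gates multi-sphere traces that apply random damage and set a status on BP_EnemyParent hits.
; An alternative projectile-spawning version is left unconnected.
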(event Custom|DeactivateFlameVFX
  (bind _mytank (Variables|Default|GetMyTank))
  (bind _weaponniagara (Variables|/Game/Blueprints/BP_PlayerCharacter.BP_PlayerCharacter_C|GetweaponNiagara _mytank))
  ;[1 1 1] deactiavte effec
  (Utilities|IsValid _weaponniagara
    (:Is%20Valid
      (Components|Activation|Deactivate _weaponniagara))))

(event Custom|ResetCoolDown
  ;[1 1 1] Play cooldown
  (Variables|Default|Setcooldown false))

(event Custom|SetCoolDown
  ;[1 1 1] Play cooldown
  (Variables|Default|Setcooldown true)
  (Utilities|Time|SetTimerbyEvent (delegate Custom|ResetCoolDown) (Variables|Default|GetfireRate)))

(event Custom|FiringEvent
  (bind _mytank (Variables|Default|GetMyTank))
  (bind _directionarrow (Variables|/Game/Blueprints/BP_PlayerCharacter.BP_PlayerCharacter_C|GetDirectionArrow _mytank))
  (bind _returnvalue (Transformation|GetWorldTransform _directionarrow))
  ;[1 1 1] Firing event (flame line traces)
  (bind _outhits (Collision|MultiSphereTraceForObjects (.location _returnvalue) (+ (.location _returnvalue) (* (Math|Vector|GetForwardVector _directionarrow) 425.0)) 5e+01 (Variables|Default|GetObject%20Types) false 0 "None"))
  (for _array_element _outhits
    (Utilities|FlowControl|Sequence
      (:then_0
        (bind _asbp_enemy_parent (Utilities|Casting|CastToBP_EnemyParent (.HitActor (Collision|BreakHitResult _array_element))))
        (Variables|/Game/StudentWork/Enemy/BP_EnemyParent.BP_EnemyParent_C|SetCurrent%20Status _asbp_enemy_parent "NewEnumerator0"))
      (:then_1
        (Game|Damage|ApplyDamage (.HitActor (Collision|BreakHitResult _array_element)) (Math|Random|RandomFloatinRange 5.0 9.0) 0 0))))
  (CallFunction|SetCoolDown))

(event EventStarted
  ;[1 1 1] Attach flame effect
  (bind _returnvalue (Niagara|SpawnSystemAttached "/Game/StudentWork/vfx/NS_Fire.NS_Fire" (Variables|/Game/Blueprints/BP_PlayerCharacter.BP_PlayerCharacter_C|GetDirectionArrow (Variables|Default|GetMyTank)) "None" "0, 0, 0" "0, 0, 0" "KeepRelativeOffset" false))
  (bind _output_get (Variables|Default|SetFlameVFX _returnvalue))
  (Variables|/Game/Blueprints/BP_PlayerCharacter.BP_PlayerCharacter_C|SetweaponNiagara (Variables|Default|GetMyTank) _output_get))

(event EventCompleted
  (bind _mytank (Variables|Default|GetMyTank))
  (bind _weaponniagara (Variables|/Game/Blueprints/BP_PlayerCharacter.BP_PlayerCharacter_C|GetweaponNiagara _mytank))
  ;[1 1 1] deactiavte effec
  (Utilities|IsValid _weaponniagara
    (:Is%20Valid
      (Components|Activation|Deactivate _weaponniagara))))

(event EventTriggered
  ;[1 1 1] initiate fire
  (if (not (Variables|Default|Getcooldown))
    (CallFunction|FiringEvent)))

(fn ConstructionScript
  (|CallParentFunction))