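; BP_LaserWeapon is a player tank weapon that damages objects with sphere traces, apparently adapted from a flame weapon.
; While off cooldown, Triggered traces from the tank's DirectionArrow to MyTank.Location, then starts a FireRate timer cooldown.
; Each hit takes damage scaled by the total hit count.
; Flame projectile and VFX spawning are disconnected, so Started does nothing and Completed only deactivates any valid FlameVFX.
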(event Custom|ResetCoolDown
  ;[1 1 1] Play cooldown
  (Variables|Default|Setcooldown false))

(event Custom|SetCoolDown
  ;[1 1 1] Play cooldown
  (Variables|Default|Setcooldown true)
  (Utilities|Time|SetTimerbyEvent (delegate Custom|ResetCoolDown) (Variables|Default|GetfireRate)))

(event Custom|FiringEvent
  (bind _mytank (Variables|Default|GetMyTank))
  ;[1 1 1] Firing event (flame line traces)
  (bind _outhits (Collision|MultiSphereTraceForObjects (Transformation|GetWorldLocation (Variables|/Game/Blueprints/BP_PlayerCharacter.BP_PlayerCharacter_C|GetDirectionArrow _mytank)) (Variables|/Game/Blueprints/BP_PlayerCharacter.BP_PlayerCharacter_C|GetLocation _mytank) 15.0 (Variables|Default|GetObject%20Types) false 0 "ForOneFrame" true "(R=1.000000,G=0.000000,B=0.750000,A=1.000000)"))
  (for _array_element _outhits
    (Game|Damage|ApplyDamage (.HitActor (Collision|BreakHitResult _array_element)) (* (Math|Conversions|ToFloat(Integer) (+ (Utilities|Array|LastIndex _outhits) 1)) 0.9) 0 0))
  (CallFunction|SetCoolDown))

(event EventStarted
  ;[1 1 1] Attach flame effect
)

(event EventCompleted
  (bind _flamevfx (Variables|Default|GetFlameVFX))
  ;[1 1 1] deactiavte effec
  (Utilities|IsValid _flamevfx
    (:Is%20Valid
      (Components|Activation|Deactivate _flamevfx))))

(event EventTriggered
  ;[1 1 1] initiate fire
  (if (not (Variables|Default|Getcooldown))
    (CallFunction|FiringEvent)))

(fn ConstructionScript
  (|CallParentFunction))