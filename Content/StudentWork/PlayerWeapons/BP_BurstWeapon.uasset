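; Burst-fire weapon for the player tank that spawns four BP_BurstProjectile shots in quick succession per trigger.
; Triggered fires only when off cooldown, and a FireRate timer clears the cooldown.
; Each shot spawns at the tank's DirectionArrow, adding MakeSpread pitch and yaw to its aim.
; MakeSpread holds a random rotator scaled by the tank's EnableRecoil, though that expression appears unconnected.
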(event Custom|EndCooldown
  ;[1 1 1] Weapon Cooldown
  (Variables|Default|Setcooldown false))

(event Custom|OnCooldown
  ;[1 1 1] Weapon Cooldown
  (Variables|Default|Setcooldown true)
  (Utilities|Time|SetTimerbyEvent (delegate Custom|EndCooldown) (Variables|Default|GetfireRate)))

(event Custom|FiringEvent
  (bind _returnvalue (Utilities|MakeSpread))
  (bind _returnvalue_2 (Utilities|MakeSpread))
  (bind _returnvalue_3 (Utilities|MakeSpread))
  (bind _returnvalue_4 (Utilities|MakeSpread))
  (bind _mytank (Variables|Default|GetMyTank))
  (bind _mytank_2 (Variables|Default|GetMyTank))
  (bind _mytank_3 (Variables|Default|GetMyTank))
  (bind _mytank_4 (Variables|Default|GetMyTank))
  (bind _directionarrow (Variables|/Game/Blueprints/BP_PlayerCharacter.BP_PlayerCharacter_C|GetDirectionArrow _mytank_4))
  (bind _directionarrow_2 (Variables|/Game/Blueprints/BP_PlayerCharacter.BP_PlayerCharacter_C|GetDirectionArrow _mytank))
  (bind _directionarrow_3 (Variables|/Game/Blueprints/BP_PlayerCharacter.BP_PlayerCharacter_C|GetDirectionArrow _mytank_2))
  (bind _directionarrow_4 (Variables|/Game/Blueprints/BP_PlayerCharacter.BP_PlayerCharacter_C|GetDirectionArrow _mytank_3))
  (bind _returnvalue_5 (Transformation|GetWorldRotation _directionarrow_2))
  (bind _returnvalue_6 (Transformation|GetWorldRotation _directionarrow_3))
  (bind _returnvalue_7 (Transformation|GetWorldRotation _directionarrow_4))
  (bind _returnvalue_8 (Transformation|GetWorldRotation _directionarrow))
  ;[1 1 1] FireEvent
  (CallFunction|OnCooldown)
  (Game|SpawnActorfromClass "/Game/StudentWork/PlayerProjectiles/BP_BurstProjectile.BP_BurstProjectile_C" (Math|Transform|MakeTransform (Transformation|GetWorldLocation _directionarrow_2) (Math|Rotator|MakeRotator 0.0 (+ (.pitch _returnvalue_5) (.pitch _returnvalue_2)) (+ (.yaw _returnvalue_5) (.yaw _returnvalue_2))) "1.000000,1.000000,1.000000") "Undefined" "MultiplyWithRoot" 0 0)
  (Utilities|FlowControl|Delay 0.02)
  (Game|SpawnActorfromClass "/Game/StudentWork/PlayerProjectiles/BP_BurstProjectile.BP_BurstProjectile_C" (Math|Transform|MakeTransform (Transformation|GetWorldLocation _directionarrow_3) (Math|Rotator|MakeRotator 0.0 (+ (.pitch _returnvalue_6) (.pitch _returnvalue_3)) (+ (.yaw _returnvalue_6) (.yaw _returnvalue_3))) "1.000000,1.000000,1.000000") "Undefined" "MultiplyWithRoot" 0 0)
  (Utilities|FlowControl|Delay 0.02)
  (Game|SpawnActorfromClass "/Game/StudentWork/PlayerProjectiles/BP_BurstProjectile.BP_BurstProjectile_C" (Math|Transform|MakeTransform (Transformation|GetWorldLocation _directionarrow_4) (Math|Rotator|MakeRotator 0.0 (+ (.pitch _returnvalue_7) (.pitch _returnvalue_4)) (+ (.yaw _returnvalue_7) (.yaw _returnvalue_4))) "1.000000,1.000000,1.000000") "Undefined" "MultiplyWithRoot" 0 0)
  (Utilities|FlowControl|Delay 0.02)
  (Game|SpawnActorfromClass "/Game/StudentWork/PlayerProjectiles/BP_BurstProjectile.BP_BurstProjectile_C" (Math|Transform|MakeTransform (Transformation|GetWorldLocation _directionarrow) (Math|Rotator|MakeRotator 0.0 (+ (.pitch _returnvalue_8) (.pitch _returnvalue)) (+ (.yaw _returnvalue_8) (.yaw _returnvalue))) "1.000000,1.000000,1.000000") "Undefined" "MultiplyWithRoot" 0 0))

(event EventTriggered
  (if (not (Variables|Default|Getcooldown))
    (CallFunction|FiringEvent)))

(fn ConstructionScript
  (|CallParentFunction))