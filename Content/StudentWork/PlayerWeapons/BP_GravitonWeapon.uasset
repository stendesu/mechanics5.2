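; BP_GravitonWeapon is a tank weapon Blueprint that fires graviton projectiles.
; The Started event fires only when off cooldown, spawning a BP_GravitonProjectile at the owning tank's direction arrow and storing a reference to it.
; Each shot sets a cooldown flag that a one-shot timer clears after FireRate seconds.
; The Triggered event is empty, so holding the input does not repeat fire.
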(event Custom|EndCooldown
  ;[1 1 1] Weapon Cooldown
  (Variables|Default|Setcooldown false))

(event Custom|OnCooldown
  ;[1 1 1] Weapon Cooldown
  (Variables|Default|Setcooldown true)
  (Utilities|Time|SetTimerbyEvent (delegate Custom|EndCooldown) (Variables|Default|GetfireRate)))

(event Custom|FiringEvent
  (bind _mytank (Variables|Default|GetMyTank))
  (bind _directionarrow (Variables|/Game/Blueprints/BP_PlayerCharacter.BP_PlayerCharacter_C|GetDirectionArrow _mytank))
  ;[1 1 1] Firing Event
  (CallFunction|OnCooldown)
  (bind _returnvalue (Game|SpawnActorfromClass "/Game/StudentWork/PlayerProjectiles/BP_GravitonProjectile.BP_GravitonProjectile_C" (Math|Transform|MakeTransform (Transformation|GetWorldLocation _directionarrow) (Transformation|GetWorldRotation _directionarrow) "1.000000,1.000000,1.000000") "Undefined" "MultiplyWithRoot" 0 0))
  (Variables|Default|SetProjectile _returnvalue))

(event EventStarted
  (if (not (Variables|Default|Getcooldown))
    (CallFunction|FiringEvent)))

(event EventTriggered)

(fn ConstructionScript
  (|CallParentFunction))