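; BP_FreezeWeapon is a tank-mounted weapon that damages enemies and sets their status, presumably to frozen.
; While triggered, a timer-based cooldown gates multi sphere traces from the tank's direction arrow to its enemy aim point.
; Each hit takes light damage, and BP_EnemyParent hits also change status.
; Flame VFX spawning and a projectile firing variant, apparently flamethrower leftovers, are unconnected.
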(event Custom|ResetCoolDown
  ;[1 1 1] Play cooldown
  (Variables|Default|Setcooldown false))

(event Custom|SetCoolDown
  ;[1 1 1] Play cooldown
  (Variables|Default|Setcooldown true)
  (Utilities|Time|SetTimerbyEvent (delegate Custom|ResetCoolDown) (Variables|Default|GetfireRate)))

(event Custom|FiringEvent
  (bind _mytank (Variables|Default|GetMyTank))
  ;[1 1 1] Firing event (flame line traces)
  (bind _outhits (Collision|MultiSphereTraceForObjects (.location (Transformation|GetWorldTransform (Variables|/Game/Blueprints/BP_PlayerCharacter.BP_PlayerCharacter_C|GetDirectionArrow _mytank))) (Variables|/Game/Blueprints/BP_PlayerCharacter.BP_PlayerCharacter_C|GetLine%20Trace%20Hit%20Location%20Enemies _mytank) 5.0 (Variables|Default|GetObject%20Types) false 0 "ForOneFrame"))
  (for _array_element _outhits
    (Utilities|FlowControl|Sequence
      (:then_0
        (bind _asbp_enemy_parent (Utilities|Casting|CastToBP_EnemyParent (.HitActor (Collision|BreakHitResult _array_element))))
        (Variables|/Game/StudentWork/Enemy/BP_EnemyParent.BP_EnemyParent_C|SetCurrent%20Status _asbp_enemy_parent "NewEnumerator1"))
      (:then_1
        (Game|Damage|ApplyDamage (.HitActor (Collision|BreakHitResult _array_element)) 0.5 0 0))))
  (CallFunction|SetCoolDown))

(event EventStarted
  ;[1 1 1] Attach flame effect
)

(event EventCompleted
  (bind _flamevfx (Variables|Default|GetFlameVFX))
  ;[1 1 1] deactiavte effec
  (Utilities|IsValid _flamevfx
    (:Is%20Valid
      (Components|Activation|Deactivate _flamevfx))))

(event EventTriggered
  ;[1 1 1] initiate fire
  (if (not (Variables|Default|Getcooldown))
    (CallFunction|FiringEvent)))

(fn ConstructionScript
  (|CallParentFunction))