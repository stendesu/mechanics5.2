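; BP_BasicEnemyNonTrackPlayer is a basic enemy that wanders and fires without any player-tracking logic.
; Move uses AIMoveTo to send it to a random reachable navmesh point around its current location.
; Attack spawns an actor at the FireArrow component's world location and rotation.
; Neither event is called within this graph, and BeginPlay, overlap and Tick are disabled stubs.
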(event EventBeginPlay
  (|CallParentFunction) ; This node is disabled and will not be called.\nDrag off pins to build functionality.
)

(event Collision|EventActorBeginOverlap
  (params (OtherActor :type Actor%20Object%20Reference))
  (|CallParentFunction OtherActor) ; This node is disabled and will not be called.\nDrag off pins to build functionality.
)

(event EventTick
  (params (DeltaSeconds :type Float%20%28single-precision%29))
  (|CallParentFunction DeltaSeconds) ; This node is disabled and will not be called.\nDrag off pins to build functionality.
)

(event EventMove
  ;[1 1 1] Move evne
  (AI|AIMoveTo self (.RandomLocation (AI|Navigation|GetRandomReachablePointinRadius (Transformation|GetActorLocation) 6e+02 0 0)) 0 5.0 false))

(event EventAttack
  (bind _firearrow (Variables|Default|GetFireArrow))
  ;[1 1 1] Attack event
  (Game|SpawnActorfromClass "/Game/StudentWork/Enemy/BP_EnemyProjectile.BP_EnemyProjectile_C" (Math|Transform|MakeTransform (Transformation|GetWorldLocation _firearrow) (Transformation|GetWorldRotation _firearrow) "1.000000,1.000000,1.000000") "Undefined" "MultiplyWithRoot" 0 0))

(fn ConstructionScript
  (|CallParentFunction))