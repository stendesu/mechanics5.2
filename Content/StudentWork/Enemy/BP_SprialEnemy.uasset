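; Spiral-shooting enemy that chases the player while its cannon head spins.
; Tick yaws the head by a fixed step each frame, so the spin speed depends on frame rate.
; Move sends it toward the player reference via AI MoveTo, Attack spawns projectiles at two fire arrows, and Death destroys it.
; Nothing in this graph calls Move, Attack or Death.
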(event Custom|RotateCannon
  (bind _head (Variables|Default|GetHead))
  ;[1 1 1] Spin cannnon
  (Transformation|SetWorldRotation _head (Math|Rotator|MakeRotator 0.0 0.0 (+ (.yaw (Transformation|GetWorldRotation _head)) 1.2)) false false))

(event EventBeginPlay
  (|CallParentFunction) ; This node is disabled and will not be called.\nDrag off pins to build functionality.
)

(event Collision|EventActorBeginOverlap
  (params (OtherActor :type Actor%20Object%20Reference))
  (|CallParentFunction OtherActor) ; This node is disabled and will not be called.\nDrag off pins to build functionality.
)

(event EventTick
  (params (DeltaSeconds :type Float%20%28single-precision%29))
  (|CallParentFunction DeltaSeconds)
  (CallFunction|RotateCannon))

(event EventMove
  (bind _playerref (Variables|Default|GetplayerREF))
  ;[1 1 1] move event
  (Utilities|IsValid _playerref
    (:Is%20Valid
      (AI|AIMoveTo self "0, 0, 0" _playerref 5.0 false))))

(event EventAttack
  (bind _firearrow (Variables|Default|GetFireArrow))
  (bind _firearrow1 (Variables|Default|GetFireArrow1))
  ;[1 1 1] Shoot even
  (Game|SpawnActorfromClass "/Game/StudentWork/Enemy/BP_EnemyProjectile_3.BP_EnemyProjectile_3_C" (Math|Transform|MakeTransform (Transformation|GetWorldLocation _firearrow) (Transformation|GetWorldRotation _firearrow) "1.000000,1.000000,1.000000") "Undefined" "MultiplyWithRoot" 0 0)
  (Game|SpawnActorfromClass "/Game/StudentWork/Enemy/BP_EnemyProjectile_3.BP_EnemyProjectile_3_C" (Math|Transform|MakeTransform (Transformation|GetWorldLocation _firearrow1) (Transformation|GetWorldRotation _firearrow1) "1.000000,1.000000,1.000000") "Undefined" "MultiplyWithRoot" 0 0))

(event EventDeath
  ;[1 1 1] Death event
  (Actor|DestroyActor))

(fn ConstructionScript
  (|CallParentFunction))