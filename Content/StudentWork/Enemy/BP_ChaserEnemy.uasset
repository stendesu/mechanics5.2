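; BP_ChaserEnemy is an enemy Blueprint that chases the player.
; Its Move event checks that PlayerREF is valid, then issues an AI MoveTo targeting that actor.
; Tick only forwards to the parent, BeginPlay and overlap nodes are disabled stubs, and nothing in this file calls Move or sets PlayerREF.
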(event EventBeginPlay
  (|CallParentFunction) ; This node is disabled and will not be called.\nDrag off pins to build functionality.
)

(event Collision|EventActorBeginOverlap
  (params (OtherActor :type Actor%20Object%20Reference))
  (|CallParentFunction OtherActor) ; This node is disabled and will not be called.\nDrag off pins to build functionality.
)

(event EventTick
  (params (DeltaSeconds :type Float%20%28single-precision%29))
  (|CallParentFunction DeltaSeconds))

(event EventMove
  (bind _playerref (Variables|Default|GetplayerREF))
  (Utilities|IsValid _playerref
    (:Is%20Valid
      (AI|AIMoveTo self "0, 0, 0" _playerref 5.0 false))))

(fn ConstructionScript
  (|CallParentFunction))