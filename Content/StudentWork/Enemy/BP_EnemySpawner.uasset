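; Enemy spawner actor that releases a one-time, staggered wave of three enemies when its linked trigger box reports an overlap.
; BeginPlay casts and caches the BP_TriggerBox reference, then Tick polls its Overlap flag behind a DoOnce.
; Each enemy class spawns with AI at a random reachable point around the spawner, separated by delays and ignoring collision.
; The spawner destroys itself after the last spawn.
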(event EventTick
  (params (DeltaSeconds :type Float%20%28single-precision%29))
  ;[1 1 1] conditions
  (bind _triggerbox (Variables|Default|GetTriggerBox)
    (:then
      (if (Variables|/Game/StudentWork/Enemy/BP_TriggerBox.BP_TriggerBox_C|Getoverlap? _triggerbox)
        (Utilities|FlowControl|DoOnce false
          (:Completed
            ;[1 1 1] spawn enemies
            (AI|SpawnAIFromClass (Variables|Default|GetenemyClass1) 0 (.RandomLocation (AI|Navigation|GetRandomReachablePointinRadius (Transformation|GetActorLocation) 5e+02 0 0)) "0, 0, 0" true 0)
            (Utilities|FlowControl|Delay 3.0)
            (AI|SpawnAIFromClass (Variables|Default|GetenemyClass2) 0 (.RandomLocation (AI|Navigation|GetRandomReachablePointinRadius (Transformation|GetActorLocation) 5e+02 0 0)) "0, 0, 0" true 0)
            (Utilities|FlowControl|Delay 3.0)
            (AI|SpawnAIFromClass (Variables|Default|GetenemyClass3) 0 (.RandomLocation (AI|Navigation|GetRandomReachablePointinRadius (Transformation|GetActorLocation) 5e+02 0 0)) "0, 0, 0" true 0)
            ;[1 1 1] clear
            (Actor|DestroyActor)))))
    (:else)))

(event EventBeginPlay
  (bind _asbp_trigger_box (Utilities|Casting|CastToBP_TriggerBox (Variables|Default|GetTriggerBoxRef)))
  (Variables|Default|SetTriggerBox _asbp_trigger_box))

(fn ConstructionScript)