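; Hammer-wielding enemy that can move toward the player and swings a spawned hammer once the player enters its attack box.
; On BeginPlay it attaches a BP_EnemyHammer to FireArrow and passes it the damage value.
; Box overlap starts a Timeline that rotates FireArrow, with a FlipFlop looping forward and reverse swings; leaving the box does not stop it.
; Death destroys both actors; stun is an empty stub.
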(event OnComponentBeginOverlap(Box)
  (params (OverlappedComponent :type Primitive%20Component%20Object%20Reference) (OtherActor :type Actor%20Object%20Reference) (OtherComp :type Primitive%20Component%20Object%20Reference) (OtherBodyIndex :type Integer) (bFromSweep :type Boolean) (SweepResult :type Hit%20Result%20Structure%20%28by%20ref%29))
  ;[1 1 1] detect player in hammerable range
  (Utilities|Casting|CastToBP_PlayerCharacter OtherActor)
  (Components|Timeline|SetPlayRate (Variables|Default|GetTimeline) 3.0)
  (CallFunction|PlayTL))

(event OnComponentEndOverlap(Box)
  (params (OverlappedComponent :type Primitive%20Component%20Object%20Reference) (OtherActor :type Actor%20Object%20Reference) (OtherComp :type Primitive%20Component%20Object%20Reference) (OtherBodyIndex :type Integer))
  ;[1 1 1] detect player in hammerable range
  (Utilities|Casting|CastToBP_PlayerCharacter OtherActor))

(event Custom|ReverseTL
  ;[1 1 1] Hammer anim and attack Timeline
  (bind _1 (Timeline|Timeline Reverse)
    (:Update
      (Transformation|SetRelativeRotation (Variables|Default|GetFireArrow) (Math|Rotator|Lerp(Rotator) "0, 0, 0" "-90.000000,0.000000,0.000000" _1) false false))
    (:Finished
      (Utilities|FlowControl|FlipFlop
        (:A
          (CallFunction|ReverseTL))
        (:B
          (CallFunction|PlayTL))))))

(event Custom|PlayTL
  ;[1 1 1] Hammer anim and attack Timeline
  (bind _1 (Timeline|Timeline Play)
    (:Update
      (Transformation|SetRelativeRotation (Variables|Default|GetFireArrow) (Math|Rotator|Lerp(Rotator) "0, 0, 0" "-90.000000,0.000000,0.000000" _1) false false))
    (:Finished
      (Utilities|FlowControl|FlipFlop
        (:A
          (CallFunction|ReverseTL))
        (:B
          (CallFunction|PlayTL))))))

(event Custom|InitiateStun
  ;[1 1 1] Stun enemy
)

(event EventBeginPlay
  (|CallParentFunction)
  ;[1 1 1] Spawn hammer
  (CallFunction|InitiateHammer))

(event Collision|EventActorBeginOverlap
  (params (OtherActor :type Actor%20Object%20Reference))
  (|CallParentFunction OtherActor) ; This node is disabled and will not be called.\nDrag off pins to build functionality.
)

(event EventTick
  (params (DeltaSeconds :type Float%20%28single-precision%29))
  (|CallParentFunction DeltaSeconds))

(event EventMove
  (bind _playerref (Variables|Default|GetplayerREF))
  ;[1 1 1] Move event
  (Utilities|IsValid _playerref
    (:Is%20Valid
      (AI|AIMoveTo self (Transformation|GetActorLocation _playerref) 0 2e+02 false))))

(event EventDeath
  ;[1 1 1] Death event
  (Actor|DestroyActor (Variables|Default|GetHammer))
  (Actor|DestroyActor))

(fn ConstructionScript
  (|CallParentFunction))

(fn InitiateHammer
  (bind _returnvalue (Game|SpawnActorfromClass "/Game/StudentWork/Enemy/BP_EnemyHammer.BP_EnemyHammer_C" (Transformation|GetWorldTransform (Variables|Default|GetFireArrow)) "Undefined" "MultiplyWithRoot" 0 0))
  (bind _output_get (Variables|Default|SetHammer _returnvalue))
  (Transformation|AttachComponentToComponent _output_get (Variables|Default|GetFireArrow) "None" "SnapToTarget" "SnapToTarget" "KeepRelative" true)
  (Variables|/Game/StudentWork/Enemy/BP_EnemyHammer.BP_EnemyHammer_C|SetBase%20Damage _output_get (Variables|Default|GetHammerDamage)))