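; Parent class for tank-style enemies, handling health, player detection and burn, freeze and stun statuses.
; Overlapping the detection volume stores the player and starts looping timers for Move and Attack, left empty like Death for children.
; Tick turns the hull toward velocity, updates the player-facing health bar and polls CurrentStatus through DoOnce gates.
; Burn and freeze spawn attached status actors, freeze slows movement, and stun briefly halts it.
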(event OnComponentBeginOverlap(playerDetection)
  (params (OverlappedComponent :type Primitive%20Component%20Object%20Reference) (OtherActor :type Actor%20Object%20Reference) (OtherComp :type Primitive%20Component%20Object%20Reference) (OtherBodyIndex :type Integer) (bFromSweep :type Boolean) (SweepResult :type Hit%20Result%20Structure%20%28by%20ref%29))
  ;[1 1 1] Detect player and Make reference
  (bind _asbp_player_character (Utilities|Casting|CastToBP_PlayerCharacter OtherActor))
  (Variables|Default|SetplayerREF _asbp_player_character)
  (CallFunction|StartMovementTimer)
  (CallFunction|StartAttackTimer))

(event Custom|Move
  ;[1 1 1] For Children
)

(event Custom|ApplyFreeze
  ;[1 1 1] Apply freeze
  (Utilities|CheckforFreeze
    (:true
      (Utilities|FlowControl|DoOnce false
        (:Completed
          (Components|Timeline|SetPlayRate (Variables|Default|GetFreezeTimer) 1.0)
          (bind _freezeref (CallFunction|ApplyStatus))
          (Timeline|FreezeTimer PlayFromStart
            (:Finished
              (Variables|Default|SetCurrent%20Status "NewEnumerator2")
              (Actor|DestroyActor _freezeref)
              (Utilities|RevertFreeze)
              (Utilities|Time|SetTimerbyEvent (delegate Custom|ResetFreeze) 4.0) ; Set cooldown before freeze again
            )))))))

(event Custom|TakeBurnDamage
  ;[1 1 1] Burn status
  (Utilities|CheckforBurn
    (:true
      (Utilities|FlowControl|DoOnce false
        (:Completed
          (bind _burnref (CallFunction|ApplyStatus))
          (Utilities|Time|SetTimerbyEvent (delegate Custom|ResetBurn) 5.0))))))

(event Custom|ResetBurn
  ;[1 1 1] Burn status
  (Variables|Default|SetCurrent%20Status "NewEnumerator2")
  (Actor|DestroyActor (stale Custom|TakeBurnDamage _burnref))
  (Utilities|FlowControl|DoOnce false) ; enters at Reset
)

(event Custom|ResetFreeze
  ;[1 1 1] Apply freeze
  (Utilities|FlowControl|DoOnce false) ; enters at Reset
)

(event Custom|FastForwardFreeze
  (bind _freezetimer (Variables|Default|GetFreezeTimer))
  ;[1 1 1] Apply freeze
  (Components|Timeline|SetPlayRate _freezetimer (+ (Components|Animation|GetPlayRate _freezetimer) 1.0)))

(event Custom|ApplyStun
  ;[1 1 1] Apply Stun
  (Utilities|CheckforStun
    (:true
      (Utilities|FlowControl|DoOnce false :!label _label
        (:Completed
          (Variables|/Script/Engine.CharacterMovementComponent|SetMaxWalkSpeed (Variables|Character|GetCharacterMovement) 0.0)
          (Utilities|FlowControl|Delay 0.7)
          (Variables|/Script/Engine.CharacterMovementComponent|SetMaxWalkSpeed (Variables|Character|GetCharacterMovement) (Variables|Default|GetDefault%20Max%20Walk%20Speed))
          (Variables|Default|SetCurrent%20Status "NewEnumerator2")
          (goto _label Reset))))))

(event Custom|AimAtPlayerCannon
  (bind _head (Variables|Default|GetHead))
  (bind _playerref (Variables|Default|GetplayerREF))
  ;[1 1 1] Aim Cannon
  (Utilities|IsValid _playerref
    (:Is%20Valid
      (Transformation|SetWorldRotation _head (Math|Rotator|FindLookatRotation (Transformation|GetWorldLocation _head) (Transformation|GetActorLocation _playerref)) false false))))

(event Custom|Attack
  ;[1 1 1] For Children
)

(event Custom|StartAttackTimer
  ;[1 1 1] AttackTimer
  (bind _returnvalue (Utilities|Time|SetTimerbyEvent (delegate Custom|Attack) (Variables|Default|GetAttackSpeed) true))
  (Variables|Default|SetAttackTimer _returnvalue))

(event Custom|StartMovementTimer
  ;[1 1 1] Move timer
  (bind _returnvalue (Utilities|Time|SetTimerbyEvent (delegate Custom|Move) (Variables|Default|GetMovementUpdateTime) true))
  (Variables|Default|SetMovementTimer _returnvalue))

(event Custom|FocusPlayer
  ;[1 1 1] Aim at Player (Arrow Only!)
)

(event Custom|Death
  ;[1 1 1] Death event
)

(event Custom|Print%20Hp
  ;[1 1 1] debug use only
  (Development|PrintString (Utilities|String|ToString(Text) (Utilities|Text|FormatText "{ENEMY NAME} HP: {HP}" (Utilities|GetDisplayName self) (Utilities|String|ToString(Float) (Variables|Default|GetCurrentHealth)))) true true "(R=0.000000,G=0.660000,B=1.000000,A=1.000000)" 0.001))

(event Custom|HullToFace
  (bind _returnvalue (Transformation|GetVelocity))
  (bind _tankbody (Variables|Default|GetTankBody))
  (bind _returnvalue_2 (Transformation|GetWorldRotation _tankbody))
  ;[1 1 1] HullToFace
  (Transformation|SetWorldRotation _tankbody (select (> (Math|Vector|VectorLength _returnvalue) 0.0) (Math|Interpolation|RInterpTo _returnvalue_2 (Math|Rotator|MakeRotator 0.0 0.0 (.yaw (Math|Rotator|MakeRotfromX _returnvalue))) (Utilities|Time|GetWorldDeltaSeconds) (Variables|Default|GetTurnRate)) _returnvalue_2) false false))

(event EventBeginPlay
  (Variables|/Script/Engine.CharacterMovementComponent|SetMaxWalkSpeed (Variables|Character|GetCharacterMovement) (Variables|Default|GetDefault%20Max%20Walk%20Speed))
  (Variables|Default|SetCurrentHealth (Variables|Default|GetMaxHealth))
  (bind _returnvalue (UserInterface|CreateWidget "/Game/StudentWork/Widgets/EnemyHpBar.EnemyHpBar_C"))
  (bind _output_get (Variables|Default|SetEnemyHpWidget _returnvalue))
  (UserInterface|SetWidget (Variables|Default|GetWidget) _output_get))

(event EventTick
  (params (DeltaSeconds :type Float%20%28single-precision%29))
  (Utilities|FlowControl|Sequence
    (:then_0
      (CallFunction|HulltoFace)
      (CallFunction|UpdateHpBarDirection)
      (CallFunction|UpdateHpBar)
      (CallFunction|PrintHp))
    (:then_1
      (CallFunction|TakeBurnDamage) ; HAS CONDITION
    )
    (:then_2
      (CallFunction|ApplyFreeze) ; HAS CONDITION
    )
    (:then_3
      (CallFunction|ApplyStun) ; HAS CONDIITOIN
    )))

(event Game|Damage|EventAnyDamage
  (params (Damage :type Float%20%28single-precision%29) (DamageType :type Damage%20Type%20Object%20Reference) (InstigatedBy :type Controller%20Object%20Reference) (DamageCauser :type Actor%20Object%20Reference))
  ;[1 1 1] Take Damage event
  (Variables|Default|SetCurrentHealth (- (Variables|Default|GetCurrentHealth) Damage))
  (if (<= (Variables|Default|GetCurrentHealth) 0.0)
    (CallFunction|Death)))

(fn ConstructionScript
  (Transformation|SetWorldRotation (Variables|Default|GetTankBody) (Transformation|GetWorldRotation (Variables|Collision|GetCapsuleComponent)) false false))

(fn ApplyStatus
  (if (Utilities|Enum|Equal(Enum) (Variables|Default|GetCurrent%20Status) "NewEnumerator0")
    (bind _returnvalue (Game|SpawnActorfromClass "/Game/StudentWork/BP_BurnStatus.BP_BurnStatus_C" (Math|Transform|MakeTransform "0, 0, 0" "0, 0, 0" "1.000000,1.000000,1.000000") "Undefined" "MultiplyWithRoot" 0 0))
    (bind _output_get (Variables|Default|SetBurnStatus _returnvalue))
    (Transformation|AttachComponentToComponent _output_get (Variables|Default|GetHead) "None" "SnapToTarget" "SnapToTarget" "SnapToTarget" true)
    (Variables|/Game/StudentWork/BP_BurnStatus.BP_BurnStatus_C|SetActorToDamage _output_get self)
    (return _output_get 0)
    (elif (Utilities|Enum|Equal(Enum) (Variables|Default|GetCurrent%20Status) "NewEnumerator1")
      (bind _returnvalue_2 (Game|SpawnActorfromClass "/Game/StudentWork/BP_FreezeStatus.BP_FreezeStatus_C" (Math|Transform|MakeTransform "0, 0, 0" "0, 0, 0" "1.000000,1.000000,1.000000") "Undefined" "MultiplyWithRoot" 0 0))
      (bind _output_get_2 (Variables|Default|SetFreezeStatus _returnvalue_2))
      (Transformation|AttachComponentToComponent _output_get_2 (Variables|Default|GetHead) "None" "SnapToTarget" "SnapToTarget" "SnapToTarget" true)
      (Variables|/Game/StudentWork/BP_FreezeStatus.BP_FreezeStatus_C|SetDamaged%20Actor _output_get_2 self)
      (Variables|/Script/Engine.CharacterMovementComponent|SetMaxWalkSpeed (Variables|Character|GetCharacterMovement) 1e+01)
      (return 0 _output_get_2))))

(fn UpdateHpBar
  (Progress|SetPercent (Variables|/Game/StudentWork/Widgets/EnemyHpBar.EnemyHpBar_C|GetProgressBar_30 (Variables|Default|GetEnemyHpWidget)) (/ (Variables|Default|GetCurrentHealth) (Variables|Default|GetMaxHealth))))

(fn UpdateHpBarDirection
  (bind _hpbardirection (Variables|Default|GetHpBarDirection))
  (bind _playerref (Variables|Default|GetplayerREF)
    (:then
      (Transformation|SetWorldRotation _hpbardirection (Math|Rotator|FindLookatRotation (Transformation|GetWorldLocation _hpbardirection) (Transformation|GetWorldLocation (Variables|/Game/Blueprints/BP_PlayerCharacter.BP_PlayerCharacter_C|GetCamera _playerref))) false false))
    (:else)))