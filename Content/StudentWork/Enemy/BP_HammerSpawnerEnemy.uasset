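; Hammer spawner enemy that shoots projectiles at the player and summons two BP_OldHammer minions once its health drops to 200, noted as half HP.
; Tick turns it toward the player via FocusPlayer and polls health, with a DoOnce gating the AI spawns at Spot1 and Spot2.
; Move picks a random reachable point nearby, and Attack fires a scaled-up BP_EnemyProjectile_2 from FireArrow.
; Death destroys both stored minions along with itself.
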(event Custom|SpawnHammers
  (bind _spot1 (Variables|Default|GetSpot1))
  (bind _spot2 (Variables|Default|GetSpot2))
  (bind _returnvalue (Transformation|GetWorldTransform _spot1))
  (bind _returnvalue_2 (Transformation|GetWorldTransform _spot2))
  ;[1 1 1] Spawn at half hp
  (if (<= (Variables|Default|GetCurrentHealth) 2e+02)
    (Utilities|FlowControl|DoOnce false
      (:Completed
        (Utilities|FlowControl|Sequence
          (:then_0
            (bind _returnvalue_3 (AI|SpawnAIFromClass "/Game/StudentWork/Enemy/BP_OldHammer.BP_OldHammer_C" 0 (.location _returnvalue) (.rotation _returnvalue) false 0))
            (Variables|Default|SetSpawnedEnemy1 _returnvalue_3))
          (:then_1
            (bind _returnvalue_4 (AI|SpawnAIFromClass "/Game/StudentWork/Enemy/BP_OldHammer.BP_OldHammer_C" 0 (.location _returnvalue_2) (.rotation _returnvalue_2) false 0))
            (Variables|Default|SetSpawnedEnemy2 _returnvalue_4)))))))

(event EventBeginPlay
  (|CallParentFunction) ; This node is disabled and will not be called.\nDrag off pins to build functionality.
)

(event Collision|EventActorBeginOverlap
  (params (OtherActor :type Actor%20Object%20Reference))
  (|CallParentFunction OtherActor) ; This node is disabled and will not be called.\nDrag off pins to build functionality.
)

(event EventTick
  (params (DeltaSeconds :type Float%20%28single-precision%29))
  (|CallParentFunction DeltaSeconds)
  (CallFunction|FocusPlayer)
  (CallFunction|SpawnHammers))

(event EventMove
  ;[1 1 1] Move evne
  (AI|AIMoveTo self (.RandomLocation (AI|Navigation|GetRandomReachablePointinRadius (Transformation|GetActorLocation) 6e+02 0 0)) 0 5.0 false))

(event EventAttack
  (bind _firearrow (Variables|Default|GetFireArrow))
  ;[1 1 1] Attack event
  (Game|SpawnActorfromClass "/Game/StudentWork/Enemy/BP_EnemyProjectile_2.BP_EnemyProjectile_2_C" (Math|Transform|MakeTransform (Transformation|GetWorldLocation _firearrow) (Transformation|GetWorldRotation _firearrow) "3.000000,3.000000,3.000000") "Undefined" "MultiplyWithRoot" 0 0))

(event EventDeath
  (Actor|DestroyActor (Variables|Default|GetSpawnedEnemy1))
  (Actor|DestroyActor))

(fn ConstructionScript
  (|CallParentFunction))