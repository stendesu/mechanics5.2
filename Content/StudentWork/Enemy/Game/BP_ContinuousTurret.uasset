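; BP_ContinuousTurret is an enemy turret that fires continuously without targeting and can be destroyed by damage.
; BeginPlay starts a looping timer at FireRate, which spawns an actor of the configured Class at the GunPoint location and rotation.
; Each AnyDamage event removes one from Hits regardless of the damage amount, and Tick destroys the turret once Hits reaches zero or below.
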(event Custom|FireProjectile
  (bind _gunpoint (Variables|Default|GetGunPoint))
  ;[1 1 1] FireProjectile
  (Game|SpawnActorfromClass (Variables|Default|GetClass) (Math|Transform|MakeTransform (Transformation|GetWorldLocation _gunpoint) (Transformation|GetWorldRotation _gunpoint) "1.000000,1.000000,1.000000") "Undefined" "MultiplyWithRoot" 0 0))

(event EventTick
  (params (DeltaSeconds :type Float%20%28single-precision%29))
  (if (<= (Variables|Default|GetHits) 0.0)
    (Actor|DestroyActor)))

(event EventBeginPlay
  ;[1 1 1] FireProjectile
  (bind _returnvalue (Utilities|Time|SetTimerbyEvent (delegate Custom|FireProjectile) (Variables|Default|GetFireRate) true))
  (Variables|Default|SetFireTimer _returnvalue))

(event Game|Damage|EventAnyDamage
  (params (Damage :type Float%20%28single-precision%29) (DamageType :type Damage%20Type%20Object%20Reference) (InstigatedBy :type Controller%20Object%20Reference) (DamageCauser :type Actor%20Object%20Reference))
  ;[1 1 1] TakeDamage
  (Variables|Default|SetHits (- (Variables|Default|GetHits) 1.0)))

(fn ConstructionScript)