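; BP_BomberEnemy is an enemy that chases the player with AIMoveTo and self-destructs on proximity.
; A player entering its detection radius stops it, speeds up its flashing material and, after a short delay, triggers DeathEvent.
; Death knocks it backwards along a timeline before calling the same DeathEvent, which clears status effects, spawns a scaled-up explosion and destroys it.
; Tick spins the tank body once health is depleted.
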(event OnComponentBeginOverlap(DetectionRadius)
  (params (OverlappedComponent :type Primitive%20Component%20Object%20Reference) (OtherActor :type Actor%20Object%20Reference) (OtherComp :type Primitive%20Component%20Object%20Reference) (OtherBodyIndex :type Integer) (bFromSweep :type Boolean) (SweepResult :type Hit%20Result%20Structure%20%28by%20ref%29))
  ;[1 1 1] SetTimer to explode
  (Utilities|Casting|CastToBP_PlayerCharacter OtherActor)
  (Variables|Default|SetCanMove? false)
  (Rendering|Material|SetMaterial (Variables|Default|GetTankBody) 1 "/Game/StudentWork/Materials/M_Flashing_Inst_FAST.M_Flashing_Inst_FAST")
  (Rendering|Material|SetMaterial (Variables|Default|GetHead) 2 "/Game/StudentWork/Materials/M_Flashing_Inst_FAST.M_Flashing_Inst_FAST")
  (Variables|/Script/Engine.CharacterMovementComponent|SetMaxWalkSpeed (Variables|Character|GetCharacterMovement) 0.0)
  (Utilities|FlowControl|Delay 0.35)
  (CallFunction|DeathEvent))

(event Custom|DeathEvent
  (bind _returnvalue (Transformation|GetActorTransform))
  ;[1 1 1] dead
  (Utilities|FlowControl|Sequence
    (:then_0
      (CallFunction|RemoveAllStatusEffects))
    (:then_1
      (Game|SpawnActorfromClass "/Game/StudentWork/BP_NaturalExplosion.BP_NaturalExplosion_C" (Math|Transform|MakeTransform (.location _returnvalue) (.rotation _returnvalue) "1.800000,1.800000,1.800000") "Undefined" "MultiplyWithRoot" 0 0)
      (Actor|DestroyActor))))

(event Custom|SpinActor
  (bind _tankbody (Variables|Default|GetTankBody))
  (bind _relativerotation (Variables|/Script/Engine.SceneComponent|GetRelativeRotation _tankbody))
  ;[1 1 1] Spinner
  (Transformation|SetRelativeRotation _tankbody (Math|Rotator|MakeRotator (.roll _relativerotation) (.pitch _relativerotation) (+ (.yaw _relativerotation) 25.0)) false false))

(event Custom|BlowBackwards
  ;[1 1 1] Send enemies backwards
  (Components|Timeline|SetPlayRate (Variables|Default|GetblowEnemyBack) 2.75)
  (bind _1 (Timeline|blowEnemyBack Play)
    (:Update
      (Transformation|SetActorLocation (Math|Vector|Lerp(Vector) (Transformation|GetActorLocation) (+ (Transformation|GetActorLocation) (* (/ (Transformation|GetActorForwardVector) -1.0) 35.0)) _1) false false))))

(event EventBeginPlay
  (|CallParentFunction) ; This node is disabled and will not be called.\nDrag off pins to build functionality.
)

(event Collision|EventActorBeginOverlap
  (params (OtherActor :type Actor%20Object%20Reference))
  (|CallParentFunction OtherActor) ; This node is disabled and will not be called.\nDrag off pins to build functionality.
)

(event EventTick
  (params (DeltaSeconds :type Float%20%28single-precision%29))
  (|CallParentFunction DeltaSeconds)
  (if (<= (Variables|Default|GetCurrentHealth) 0.0)
    (CallFunction|SpinActor)))

(event EventMove
  (if (Variables|Default|GetCanMove?)
    (Rendering|Material|SetMaterial (Variables|Default|GetTankBody) 1 "/Game/StudentWork/Materials/M_Flashing_Inst_RED.M_Flashing_Inst_RED")
    (AI|AIMoveTo self "0, 0, 0" (Variables|Default|GetplayerREF) 5.0 false)))

(event EventDeath
  ;[1 1 1] Initiate death
  (Variables|Default|SetCanMove? false)
  (Variables|/Script/Engine.CharacterMovementComponent|SetMaxWalkSpeed (Variables|Character|GetCharacterMovement) 0.0)
  (CallFunction|BlowBackwards)
  (Utilities|FlowControl|Delay 0.285714)
  (CallFunction|DeathEvent))

(fn ConstructionScript
  (|CallParentFunction))