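; Charge-up tank enemy that aims at the player each tick, approaches them, then roams to a random nearby point.
; Its attack grows a charge sphere on a timeline, then knocks the tank backwards along its head's axis and fires a projectile if still alive.
; On death it runs once, stopping movement and starting a staggered red emissive material swap, then spawns an explosion and destroys itself after a short delay.
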(event Custom|PlayTL
  (bind _firearrow (Variables|Default|GetFireArrow))
  ;[1 1 1] Charge up buulet
  ;;[1 1 1] set sphere size
  (bind _newtrack_0 (Timeline|ChargeBullet PlayFromStart)
    (:Update
      (Transformation|SetRelativeScale3D (Variables|Default|GetPrepareFireVisuAL) (Math|Vector|Lerp(Vector) "0, 0, 0" "10.000000,10.000000,10.000000" _newtrack_0)))
    (:Finished
      (CallFunction|BlowBackwards)
      (if (not (<= (Variables|Default|GetCurrentHealth) 0.0))
        (Game|SpawnActorfromClass "/Game/StudentWork/Enemy/Projectiles/BP_ChargeEnemyProjectile.BP_ChargeEnemyProjectile_C" (Math|Transform|MakeTransform (Transformation|GetWorldLocation _firearrow) (Transformation|GetWorldRotation _firearrow) "1.000000,1.000000,1.000000") "Undefined" "MultiplyWithRoot" 0 0)))))

(event Custom|BlowBackwards
  ;[1 1 1] Send enemies backwards
  (Components|Timeline|SetPlayRate (Variables|Default|GetblowEnemyBack) 5.0)
  (bind _1 (Timeline|BlowEnemyBack PlayFromStart)
    (:Update
      (Transformation|SetActorLocation (Math|Vector|Lerp(Vector) (Transformation|GetActorLocation) (+ (Transformation|GetActorLocation) (* (/ (Math|Vector|GetForwardVector (Variables|Default|GetHead)) -1.0) 12.0)) _1) false false))
    (:Finished
      ;[1 1 1] ResetAttack
      (Transformation|SetRelativeScale3D (Variables|Default|GetPrepareFireVisuAL) "0, 0, 0"))))

(event Custom|IntiateSelfDestruct
  (bind _tankbody (Variables|Default|GetTankBody))
  ;[1 1 1] self destruct
  (Variables|/Script/Engine.CharacterMovementComponent|SetMaxWalkSpeed (Variables|Character|GetCharacterMovement) 0.0)
  (Rendering|Material|SetMaterial _tankbody 0 "/Game/Materials/MI_Emissive_Red_2.MI_Emissive_Red_2")
  (Utilities|FlowControl|Delay 1.0)
  (Rendering|Material|SetMaterial _tankbody 1 "/Game/Materials/MI_EmissiveRed.MI_EmissiveRed")
  (Utilities|FlowControl|Delay 1.0)
  (Rendering|Material|SetMaterial _tankbody 2 "/Game/Materials/MI_Emissive_Red_2.MI_Emissive_Red_2"))

(event EventBeginPlay
  (|CallParentFunction) ; This node is disabled and will not be called.\nDrag off pins to build functionality.
)

(event Collision|EventActorBeginOverlap
  (params (OtherActor :type Actor%20Object%20Reference))
  (|CallParentFunction OtherActor) ; This node is disabled and will not be called.\nDrag off pins to build functionality.
)

(event EventTick
  (params (DeltaSeconds :type Float%20%28single-precision%29))
  (|CallParentFunction DeltaSeconds)
  (CallFunction|AimatPlayerCannon))

(event EventMove
  (bind _self self)
  ;[1 1 1] go to player
  (AI|AIMoveTo _self (Transformation|GetActorLocation (Variables|Default|GetplayerREF)) 0 1.5e+03 false
    (:OnSuccess
      ;[1 1 1] roam
      (AI|AIMoveTo _self (.RandomLocation (AI|Navigation|GetRandomReachablePointinRadius (Transformation|GetActorLocation) 6e+02 0 0)) 0 5.0 false))))

(event EventAttack
  (CallFunction|PlayTL))

(event EventDeath
  ;[1 1 1] DeathEvent
  (Utilities|FlowControl|DoOnce false
    (:Completed
      (CallFunction|IntiateSelfDestruct)
      (Utilities|FlowControl|Delay 1.0)
      (Game|SpawnActorfromClass "/Game/StudentWork/BP_NaturalExplosion.BP_NaturalExplosion_C" (Math|Transform|MakeTransform (Transformation|GetActorLocation) "0, 0, 0" "1.200000,1.200000,1.200000") "Undefined" "MultiplyWithRoot" 0 0)
      (Actor|DestroyActor))))

(fn ConstructionScript
  (|CallParentFunction))