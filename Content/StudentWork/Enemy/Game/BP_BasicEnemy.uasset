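; Basic AI enemy that closes on the player, roams and fires projectiles, built on a parent enemy class.
; Move pathfinds to within range of the player, then on success walks to a random reachable point near itself.
; Tick aims at the player through AimAtPlayerCannon and re-randomizes AttackSpeed every frame.
; Attack spawns BP_EnemyProjectile from FireArrow, and Death clears status effects before destroying the actor.
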(event EventBeginPlay
  (|CallParentFunction))

(event Collision|EventActorBeginOverlap
  (params (OtherActor :type Actor%20Object%20Reference))
  (|CallParentFunction OtherActor))

(event EventTick
  (params (DeltaSeconds :type Float%20%28single-precision%29))
  (|CallParentFunction DeltaSeconds)
  (CallFunction|AimatPlayerCannon)
  (Variables|Default|SetAttackSpeed (Math|Random|RandomFloatinRange 1.2 3.6)))

(event EventMove
  (bind _self self)
  ;[1 1 1] go to player
  (AI|AIMoveTo _self (Transformation|GetActorLocation (Variables|Default|GetplayerREF)) 0 1.2e+03 false
    (:OnSuccess
      ;[1 1 1] roam
      (AI|AIMoveTo _self (.RandomLocation (AI|Navigation|GetRandomReachablePointinRadius (Transformation|GetActorLocation) 6e+02 0 0)) 0 5.0 false))))

(event EventAttack
  (bind _firearrow (Variables|Default|GetFireArrow))
  ;[1 1 1] Attack event
  (Game|SpawnActorfromClass "/Game/StudentWork/Enemy/BP_EnemyProjectile.BP_EnemyProjectile_C" (Math|Transform|MakeTransform (Transformation|GetWorldLocation _firearrow) (Transformation|GetWorldRotation _firearrow) "1.000000,1.000000,1.000000") "Undefined" "MultiplyWithRoot" 0 0))

(event EventDeath
  (Utilities|FlowControl|Sequence
    (:then_0
      (CallFunction|RemoveAllStatusEffects))
    (:then_1
      (Actor|DestroyActor))))

(fn ConstructionScript
  (|CallParentFunction))