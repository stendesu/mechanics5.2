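; Boss enemy Blueprint that adds health-based phases to its parent and triggers the player's end screen on death.
; Each Tick runs a nested chain of health percentage checks from lowest threshold to highest.
; Only the 55 percent branch acts, setting walk speed once; the other thresholds are empty.
; The comparison inside CheckHealthPercent appears as unused, not connected to a return value.
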(event Custom|HealthThresholdEvents
  (if (not (Utilities|CheckHealthPercent 1e+01))
    (if (not (Utilities|CheckHealthPercent 25.0))
      (if (not (Utilities|CheckHealthPercent 4e+01))
        (if (Utilities|CheckHealthPercent 55.0)
          (Utilities|FlowControl|DoOnce false
            (:Completed
              (bind _output_get (Variables|Default|SetDefault%20Max%20Walk%20Speed 6.4e+02))
              (Variables|/Script/Engine.CharacterMovementComponent|SetMaxWalkSpeed (Variables|Character|GetCharacterMovement) _output_get)))
          (elif (not (Utilities|CheckHealthPercent 7e+01))
            (if (Utilities|CheckHealthPercent 85.0)
              _)))))))

(event EventBeginPlay
  (|CallParentFunction) ; This node is disabled and will not be called.\nDrag off pins to build functionality.
)

(event Collision|EventActorBeginOverlap
  (params (OtherActor :type Actor%20Object%20Reference)))

(event EventTick
  (params (DeltaSeconds :type Float%20%28single-precision%29))
  (|CallParentFunction DeltaSeconds)
  (CallFunction|HealthThresholdEvents))

(event EventDeath
  (Default|CallEndScreen (Variables|Default|GetplayerREF)))

(fn ConstructionScript
  (|CallParentFunction))