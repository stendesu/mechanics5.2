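; Enemy mortar turret that fires at a linked BP_MortarTarget, cached from its fire target and destroyed along with the turret on death.
; Attack spawns a visible mortar projectile at the fire arrow and plays a timeline that scales the cannon for recoil.
; After a short delay it tells the target actor to spawn its own projectile, splitting each shot between launch and impact ends.
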(event Custom|CannonRecoilTL
  ;[1 1 1] CannonAnim
  (bind _newtrack_0 (Timeline|mortarChargeTL PlayFromStart)
    (:Update
      (Transformation|SetWorldScale3D (Variables|Default|GetCannon) (Math|Vector|Lerp(Vector) "1.000000,1.000000,0.900000" "1.000000,1.000000,0.400000" _newtrack_0)))))

(event EventBeginPlay
  (|CallParentFunction)
  ;[1 1 1] Set timeline play rate
  (Components|Timeline|SetPlayRate (Variables|Default|GetmortarChargeTL) 4.0)
  ;[1 1 1] Get target reference
  (bind _asbp_mortar_target (Utilities|Casting|CastToBP_MortarTarget (Variables|Default|GetFireTarget)))
  (Variables|Default|SetAs%20BP%20Mortar%20Target _asbp_mortar_target)
  ;[1 1 1] make it bigger
  (Transformation|SetActorScale3D "1.500000,1.500000,1.500000"))

(event Collision|EventActorBeginOverlap
  (params (OtherActor :type Actor%20Object%20Reference))
  (|CallParentFunction OtherActor) ; This node is disabled and will not be called.\nDrag off pins to build functionality.
)

(event EventTick
  (params (DeltaSeconds :type Float%20%28single-precision%29))
  (|CallParentFunction DeltaSeconds) ; This node is disabled and will not be called.\nDrag off pins to build functionality.
)

(event EventAttack
  (bind _firearrow (Variables|Default|GetFireArrow))
  (bind _as_bp_mortar_target (Variables|Default|GetAs%20BP%20Mortar%20Target))
  ;[1 1 1] Attackevent
  (Game|SpawnActorfromClass "/Game/StudentWork/Enemy/Projectiles/BP_MortarProjectile.BP_MortarProjectile_C" (Math|Transform|MakeTransform (Transformation|GetWorldLocation _firearrow) (Transformation|GetWorldRotation _firearrow) "1.000000,1.000000,1.000000") "Undefined" "MultiplyWithRoot" 0 0)
  (CallFunction|CannonRecoilTL)
  (Utilities|FlowControl|Delay 1.0)
  (Utilities|IsValid _as_bp_mortar_target
    (:Is%20Valid
      (Default|SpawnProjectile _as_bp_mortar_target))))

(event EventDeath
  ;[1 1 1] Death event
  (Actor|DestroyActor (Variables|Default|GetAs%20BP%20Mortar%20Target))
  (Utilities|FlowControl|Sequence
    (:then_0
      (CallFunction|RemoveAllStatusEffects))
    (:then_1
      (Actor|DestroyActor))))

(fn ConstructionScript
  (|CallParentFunction))