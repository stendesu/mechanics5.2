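; BP_DetectTurret is an enemy turret that aims at the player within its detection volume and can be destroyed.
; A looping timer started at BeginPlay spawns projectiles from BarrelArrow every FireRate seconds, whether or not the player is detected.
; CheckForPlayer overlaps set SeePlayer, letting Tick call TrackPlayer to rotate only BarrelArrow toward the player.
; Each damage event removes one hit regardless of amount, and Tick destroys the turret at zero.
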(event OnComponentBeginOverlap(CheckForPlayer)
  (params (OverlappedComponent :type Primitive%20Component%20Object%20Reference) (OtherActor :type Actor%20Object%20Reference) (OtherComp :type Primitive%20Component%20Object%20Reference) (OtherBodyIndex :type Integer) (bFromSweep :type Boolean) (SweepResult :type Hit%20Result%20Structure%20%28by%20ref%29))
  (bind _asbp_player_character (Utilities|Casting|CastToBP_PlayerCharacter OtherActor))
  (Variables|Default|SetPlayerRef _asbp_player_character)
  (Variables|Default|SetSeePlayer? true))

(event OnComponentEndOverlap(CheckForPlayer)
  (params (OverlappedComponent :type Primitive%20Component%20Object%20Reference) (OtherActor :type Actor%20Object%20Reference) (OtherComp :type Primitive%20Component%20Object%20Reference) (OtherBodyIndex :type Integer))
  (bind _asbp_player_character (Utilities|Casting|CastToBP_PlayerCharacter OtherActor))
  (Variables|Default|SetPlayerRef _asbp_player_character)
  (Variables|Default|SetSeePlayer? false))

(event Custom|FireProjectile
  (bind _barrelarrow (Variables|Default|GetBarrelArrow))
  ;[1 1 1] FireProjectile
  (Game|SpawnActorfromClass (Variables|Default|GetClass) (Math|Transform|MakeTransform (Transformation|GetWorldLocation _barrelarrow) (Transformation|GetWorldRotation _barrelarrow) "1.000000,1.000000,1.000000") "Undefined" "MultiplyWithRoot" 0 0))

(event EventTick
  (params (DeltaSeconds :type Float%20%28single-precision%29))
  (if (<= (Variables|Default|GetHits) 0.0)
    (Actor|DestroyActor)
    (elif (Variables|Default|GetSeePlayer?)
      (CallFunction|TrackPlayer))))

(event EventBeginPlay
  ;[1 1 1] FireProjectile
  (bind _returnvalue (Utilities|Time|SetTimerbyEvent (delegate Custom|FireProjectile) (Variables|Default|GetFireRate) true))
  (Variables|Default|SetFireTimer _returnvalue))

(event Game|Damage|EventAnyDamage
  (params (Damage :type Float%20%28single-precision%29) (DamageType :type Damage%20Type%20Object%20Reference) (InstigatedBy :type Controller%20Object%20Reference) (DamageCauser :type Actor%20Object%20Reference))
  ;[1 1 1] TakeDamage
  (Variables|Default|SetHits (- (Variables|Default|GetHits) 1.0)))

(fn ConstructionScript)

(fn TrackPlayer
  (bind _barrelarrow (Variables|Default|GetBarrelArrow))
  (bind _playerref (Variables|Default|GetplayerREF))
  (Utilities|IsValid _playerref
    (:Is%20Valid
      (Transformation|SetWorldRotation _barrelarrow (Math|Rotator|FindLookatRotation (Transformation|GetWorldLocation _barrelarrow) (Transformation|GetActorLocation _playerref)) false false))))