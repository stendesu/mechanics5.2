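; Melee enemy Blueprint that chases the player and swings a spawned hammer when within reach.
; On BeginPlay it spawns BP_EnemyHammer, attaches it to FireArrow and passes it the damage value.
; Each tick it updates player distance, turns the head toward the player, and either issues AI MoveTo or attacks.
; The attack is a timeline rotating FireArrow, gated by a state enum that resets after a cooldown delay.
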(event Custom|HammerMoveTo
  (bind _reachplayerdistance (Variables|Default|GetreachPlayerDistance))
  (if (<= (Math|Conversions|ToFloat(Integer) (Math|Float|Round (Variables|Default|GetcurrentPlayerDistance))) _reachplayerdistance)
    (CallFunction|HammerAnim)
    (else
      ;[1 1 1] go to player
      (AI|AIMoveTo self (Transformation|GetActorLocation (Variables|Default|GetplayerREF)) 0 _reachplayerdistance false))))

(event Custom|hammerLookAtPlayer
  (bind _head (Variables|Default|GetHead))
  (bind _playerref (Variables|Default|GetplayerREF))
  (bind _returnvalue (Transformation|GetActorLocation _playerref))
  (bind _returnvalue_2 (Transformation|GetWorldLocation _head))
  (bind _returnvalue_3 (Math|Rotator|FindLookatRotation _returnvalue_2 _returnvalue))
  ;[1 1 1] look at player
  (Utilities|IsValid _playerref
    (:Is%20Valid
      (Transformation|SetWorldRotation _head (Math|Rotator|MakeRotator (.roll _returnvalue_3) 0.0 (.yaw _returnvalue_3)) false false))))

(event Custom|GetDistanceToPlayer
  ;[1 1 1] FindDistanceBetweenPlayer
  (Variables|Default|SetcurrentPlayerDistance (Math|Vector|VectorLength (- (Transformation|GetActorLocation (Variables|Default|GetplayerREF)) (Transformation|GetActorLocation)))))

(event Custom|HammerAnim
  (if (not (Utilities|Enum|Equal(Enum) (Variables|Default|GetcurrentHammerState) "NewEnumerator2"))
    (Variables|Default|SetcurrentHammerState "NewEnumerator2")
    (bind _arrowrot (Timeline|HammerAnimTL PlayFromStart)
      (:Update
        (Transformation|SetRelativeRotation (Variables|Default|GetFireArrow) (Math|Rotator|Lerp(Rotator) "0, 0, 0" "-90.000000,0.000000,0.000000" _arrowrot true) false false))
      (:Finished
        (Utilities|FlowControl|Delay (Variables|Default|GetattackCooldown))
        (Variables|Default|SetcurrentHammerState "NewEnumerator3")))))

(event EventBeginPlay
  (|CallParentFunction)
  (CallFunction|InitiateHammer)
  (Variables|Default|SetcurrentHammerState "NewEnumerator0"))

(event EventTick
  (params (DeltaSeconds :type Float%20%28single-precision%29))
  (|CallParentFunction DeltaSeconds)
  (CallFunction|HammerMoveto)
  (CallFunction|HammerLookatPlayer)
  (CallFunction|GetDistancetoPlayer))

(fn ConstructionScript
  (|CallParentFunction))

(fn InitiateHammer
  (bind _returnvalue (Game|SpawnActorfromClass "/Game/StudentWork/Enemy/BP_EnemyHammer.BP_EnemyHammer_C" (Transformation|GetWorldTransform (Variables|Default|GetFireArrow)) "Undefined" "MultiplyWithRoot" 0 0))
  (bind _output_get (Variables|Default|SetHammer _returnvalue))
  (Transformation|AttachComponentToComponent _output_get (Variables|Default|GetFireArrow) "None" "SnapToTarget" "SnapToTarget" "KeepRelative" true)
  (Variables|/Game/StudentWork/Enemy/BP_EnemyHammer.BP_EnemyHammer_C|SetBase%20Damage _output_get (Variables|Default|GetHammer%20Damage)))