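; BP_HealthPack is a health pickup that spins and floats between its start location and an offset.
; A timeline lerps its position, with a FlipFlop on finish alternating reverse and play, while Tick adds a frame-rate-dependent rotation.
; On mesh overlap, a BP_PlayerCharacter below full health gains a fixed amount capped at max, its health bar updates, and the pack destroys itself.
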(event OnComponentBeginOverlap(StaticMesh)
  (params (OverlappedComponent :type Primitive%20Component%20Object%20Reference) (OtherActor :type Actor%20Object%20Reference) (OtherComp :type Primitive%20Component%20Object%20Reference) (OtherBodyIndex :type Integer) (bFromSweep :type Boolean) (SweepResult :type Hit%20Result%20Structure%20%28by%20ref%29))
  (bind _asbp_player_character (Utilities|Casting|CastToBP_PlayerCharacter OtherActor))
  ;[1 1 1] isPlayerFullHp?
  (if (not (>= (Variables|/Game/Blueprints/BP_PlayerCharacter.BP_PlayerCharacter_C|GetCurrentHealth _asbp_player_character) (Variables|/Game/Blueprints/BP_PlayerCharacter.BP_PlayerCharacter_C|GetMaxHealth _asbp_player_character)))
    ;[1 1 1] GiveHealth
    (if (>= (+ (Variables|/Game/Blueprints/BP_PlayerCharacter.BP_PlayerCharacter_C|GetCurrentHealth _asbp_player_character) 3e+01) (Variables|/Game/Blueprints/BP_PlayerCharacter.BP_PlayerCharacter_C|GetMaxHealth _asbp_player_character))
      (Variables|/Game/Blueprints/BP_PlayerCharacter.BP_PlayerCharacter_C|SetCurrentHealth _asbp_player_character (Variables|/Game/Blueprints/BP_PlayerCharacter.BP_PlayerCharacter_C|GetMaxHealth _asbp_player_character))
      (else
        (Variables|/Game/Blueprints/BP_PlayerCharacter.BP_PlayerCharacter_C|SetCurrentHealth _asbp_player_character (+ (Variables|/Game/Blueprints/BP_PlayerCharacter.BP_PlayerCharacter_C|GetCurrentHealth _asbp_player_character) 3e+01))))
    ;;[1 1 1] update healthbar
    (CallFunction|UpdatePlayerHealthBar)
    (Actor|DestroyActor)))

(event Custom|ReverseTl
  ;[1 1 1] Float&RotationEffect
  (bind _tack1 (Timeline|floatTL Reverse)
    (:Update
      (Transformation|SetActorLocation (Math|Vector|Lerp(Vector) (Variables|Default|GetstartLocation) (+ (Variables|Default|GetstartLocation) (Variables|Default|GettargetLocation)) _tack1) false false))
    (:Finished
      (Utilities|FlowControl|FlipFlop
        (:A
          (CallFunction|ReverseTl))
        (:B
          (CallFunction|PlayTl))))))

(event Custom|PlayTl
  ;[1 1 1] Float&RotationEffect
  (bind _tack1 (Timeline|floatTL Play)
    (:Update
      (Transformation|SetActorLocation (Math|Vector|Lerp(Vector) (Variables|Default|GetstartLocation) (+ (Variables|Default|GetstartLocation) (Variables|Default|GettargetLocation)) _tack1) false false))
    (:Finished
      (Utilities|FlowControl|FlipFlop
        (:A
          (CallFunction|ReverseTl))
        (:B
          (CallFunction|PlayTl))))))

(event Custom|UpdatePlayerHealthBar
  (Default|UpdateHealth (Variables|/Game/Blueprints/BP_PlayerCharacter.BP_PlayerCharacter_C|GetMyUI (stale OnComponentBeginOverlap(StaticMesh) _asbp_player_character))))

(event EventBeginPlay
  ;[1 1 1] SaveStartLocatio&Initiate
  (Variables|Default|SetstartLocation (Transformation|GetActorLocation))
  (CallFunction|PlayTl))

(event EventTick
  (params (DeltaSeconds :type Float%20%28single-precision%29))
  ;[1 1 1] RotationEffect
  (Class|Actor|AddActorWorldRotation "0.000000,0.500000,0.000000"))

(fn ConstructionScript)